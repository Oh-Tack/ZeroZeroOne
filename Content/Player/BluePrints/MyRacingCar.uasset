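; Player Chaos racing car that adds drift torque handling and shows race results through BP_RaceManager events.
; While DriftKeyPressed, Tick calls Torq to set wheel 2 and 3 drive torque from throttle and per-gear values, and raises angular damping when airborne.
; Player finish creates the result widget, and each racer finish refreshes it.
; Throttle, brake, steer and look input events are empty, with their handler logic left disconnected.
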(event `OnRacerFinished`
  (params (Record :type "FinishRecord Structure (by ref)"))
  (bind _raceresult (`self.RaceResult`))
  (`/Engine/EditorBlueprintResources/StandardMacros.IsValid` _raceresult
    (:`Is Valid`
      (`/Game/UI/WBP_RaceResult.RefreshResult` _raceresult))))

(event `OnPlayerFinished_Event`
  (params (PlayerVehicle :type "Actor Object Reference"))
  (bind _returnvalue (`|CreateWidget` "/Game/UI/WBP_RaceResult.WBP_RaceResult_C"))
  (bind _output_get (set `self.RaceResult` _returnvalue))
  (`UserWidget.AddToViewport` _output_get 0))

(event `self.ReceiveBeginPlay`
  (bind _returnvalue (`GameplayStatics.GetActorOfClass` "/Game/AI/BP_RaceManager.BP_RaceManager_C"))
  (bind _output_get (set `self.RaceManager` _returnvalue))
  (add `CPP_AIRaceManager.OnPlayerFinished` _output_get (`|CreateDelegate` :!event `OnPlayerFinished_Event`))
  (add `CPP_AIRaceManager.OnRacerFinished` _output_get (`|CreateDelegate` :!event `OnRacerFinished`)))

(event `self.ReceiveTick`
  (params (DeltaSeconds :type "Float (single-precision)"))
  (if (`self.bDriftKeyPressed`)
    (`self.Torq`)
    (`PrimitiveComponent.SetAngularDamping` (`self.Mesh`) (`KismetMathLibrary.SelectFloat` 0.0 3.0 (`NavMovementComponent.IsMovingOnGround` (`self.ChaosMovement`))))))

(event `EnhancedInput|/Game/Player/Inputs/IA_LookAround`
  (params (ActionValue :type "Float (double-precision)") (ElapsedSeconds :type "Float (double-precision)") (TriggeredSeconds :type "Float (double-precision)") (InputAction :type "InputAction Object Reference" :default "/Game/Player/Inputs/IA_LookAround.IA_LookAround")))

(event `EnhancedInput|/Game/Player/Inputs/IA_Throttle`
  (params (ActionValue :type "Float (double-precision)") (ElapsedSeconds :type "Float (double-precision)") (TriggeredSeconds :type "Float (double-precision)") (InputAction :type "InputAction Object Reference" :default "/Game/Player/Inputs/IA_Throttle.IA_Throttle")))

(event `EnhancedInput|/Game/Player/Inputs/IA_Brake`
  (params (ActionValue :type "Float (double-precision)") (ElapsedSeconds :type "Float (double-precision)") (TriggeredSeconds :type "Float (double-precision)") (InputAction :type "InputAction Object Reference" :default "/Game/Player/Inputs/IA_Brake.IA_Brake")))

(event `EnhancedInput|/Game/Player/Inputs/IA_Steer`
  (params (ActionValue :type "Float (double-precision)") (ElapsedSeconds :type "Float (double-precision)") (TriggeredSeconds :type "Float (double-precision)") (InputAction :type "InputAction Object Reference" :default "/Game/Player/Inputs/IA_Steer.IA_Steer")))

(fn `Torq`
  (bind _chaosmovement (`self.ChaosMovement`))
  (bind _chaosmovement_2 (`self.ChaosMovement`))
  (bind _chaosmovement_3 (`self.ChaosMovement`))
  (bind _chaosmovement_4 (`self.ChaosMovement`))
  (bind _chaosmovement_5 (`self.ChaosMovement`))
  (bind _chaosmovement_6 (`self.ChaosMovement`))
  (if (>= (`ChaosVehicleMovementComponent.GetTargetGear` (`self.ChaosMovement`)) 1)
    (if (== (`ChaosVehicleMovementComponent.GetTargetGear` (`self.ChaosMovement`)) 1)
      (bind _returnvalue (`ChaosVehicleMovementComponent.GetThrottleInput` (`self.ChaosMovement`)))
      (bind _returnvalue_2 (* (* _returnvalue (`self.TorqueMuliplier`)) (`self.FirstGearTorque`)))
      (`ChaosWheeledVehicleMovementComponent.SetDriveTorque` _chaosmovement _returnvalue_2 2)
      (`ChaosWheeledVehicleMovementComponent.SetDriveTorque` _chaosmovement _returnvalue_2 3)
      (elif (== (`ChaosVehicleMovementComponent.GetTargetGear` (`self.ChaosMovement`)) 2)
        (bind _returnvalue_3 (`ChaosVehicleMovementComponent.GetThrottleInput` (`self.ChaosMovement`)))
        (bind _returnvalue_4 (* (* _returnvalue_3 (`self.TorqueMuliplier`)) (`self.SecondGearTorque`)))
        (`ChaosWheeledVehicleMovementComponent.SetDriveTorque` _chaosmovement_2 _returnvalue_4 2)
        (`ChaosWheeledVehicleMovementComponent.SetDriveTorque` _chaosmovement_2 _returnvalue_4 3)
        (elif (== (`ChaosVehicleMovementComponent.GetTargetGear` (`self.ChaosMovement`)) 3)
          (bind _returnvalue_5 (`ChaosVehicleMovementComponent.GetThrottleInput` (`self.ChaosMovement`)))
          (bind _returnvalue_6 (* (* _returnvalue_5 (`self.TorqueMuliplier`)) (`self.ThirdGearTorque`)))
          (`ChaosWheeledVehicleMovementComponent.SetDriveTorque` _chaosmovement_3 _returnvalue_6 2)
          (`ChaosWheeledVehicleMovementComponent.SetDriveTorque` _chaosmovement_3 _returnvalue_6 3)
          (elif (== (`ChaosVehicleMovementComponent.GetTargetGear` (`self.ChaosMovement`)) 4)
            (bind _returnvalue_7 (`ChaosVehicleMovementComponent.GetThrottleInput` (`self.ChaosMovement`)))
            (bind _returnvalue_8 (* (* _returnvalue_7 (`self.TorqueMuliplier`)) (`self.FourthGearTorque`)))
            (`ChaosWheeledVehicleMovementComponent.SetDriveTorque` _chaosmovement_4 _returnvalue_8 2)
            (`ChaosWheeledVehicleMovementComponent.SetDriveTorque` _chaosmovement_4 _returnvalue_8 3)
            (elif (== (`ChaosVehicleMovementComponent.GetTargetGear` (`self.ChaosMovement`)) 5)
              (bind _returnvalue_9 (`ChaosVehicleMovementComponent.GetThrottleInput` (`self.ChaosMovement`)))
              (bind _returnvalue_10 (* (* _returnvalue_9 (`self.TorqueMuliplier`)) (`self.FifthGearTorque`)))
              (`ChaosWheeledVehicleMovementComponent.SetDriveTorque` _chaosmovement_5 _returnvalue_10 2)
              (`ChaosWheeledVehicleMovementComponent.SetDriveTorque` _chaosmovement_5 _returnvalue_10 3))))))
    (else
      (bind _returnvalue_11 (`ChaosVehicleMovementComponent.GetThrottleInput` (`self.ChaosMovement`)))
      (bind _returnvalue_12 (* _returnvalue_11 1.0))
      (`ChaosWheeledVehicleMovementComponent.SetDriveTorque` _chaosmovement_6 _returnvalue_12 2)
      (`ChaosWheeledVehicleMovementComponent.SetDriveTorque` _chaosmovement_6 _returnvalue_12 3))))

(fn `UserConstructionScript`)